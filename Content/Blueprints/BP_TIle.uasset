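; Grid tile actor that takes a square, pointy-top hexagon or flat-top hexagon shape and shows a selected color on interaction.
; Initialize swaps the mesh, attaches the tile to its owner and sets its relative location from Row and Column.
; Spacing derives from mesh bounds, with hexagons using three-quarter steps and half-tile offsets on odd rows or columns.
; A dynamic material instance drives the color, which OnInteract toggles between normal and selected.
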(event EventBeginPlay
  (CallFunction|CreateMID))

(event Collision|EventActorBeginOverlap
  (params (OtherActor :type Actor%20Object%20Reference)))

(event EventTick
  (params (DeltaSeconds :type Float%20%28single-precision%29)))

(fn ConstructionScript)

(fn Initialize
  (params (InType :type EGridType%20Enum :default "NewEnumerator0"))
  (bind _returnvalue (Components|GetOwner))
  (Utilities|IsValid _returnvalue
    (:Is%20Valid
      (CallFunction|SetMesh InType)
      (Transformation|AttachActorToActor _returnvalue "None" "SnapToTarget" "SnapToTarget" "KeepRelative" false)
      (bind _outlocation (CallFunction|CalculateLocation InType))
      (Transformation|SetActorRelativeLocation _outlocation))))

(fn SetMesh
  (params (InType :type EGridType%20Enum :default "NewEnumerator0"))
  (Components|StaticMesh|SetStaticMesh (Variables|Default|GetTile) (Utilities|Select :Index InType :NewEnumerator0 "/Game/Meshes/SM_Tile.SM_Tile" :NewEnumerator1 "/Game/Meshes/Hexagon_P_Top.Hexagon_P_Top" :NewEnumerator2 "/Game/Meshes/Hexagon_F_Top.Hexagon_F_Top"))
  (CallFunction|CreateMID))

(fn CalculateLocation
  (params (InType :type EGridType%20Enum :default "NewEnumerator0"))
  (bind _tile (Variables|Default|GetTile))
  (bind _column (Variables|Default|GetColumn))
  (bind _row (Variables|Default|GetRow))
  (bind _boxextent (Collision|GetComponentBounds _tile))
  (bind (_x _y) (Math|Vector|BreakVector _boxextent))
  (bind _returnvalue (* _y 2.0 _row))
  (bind _returnvalue_2 (* _x 2.0 _column))
  (return (Utilities|Select :Index InType :NewEnumerator0 (Math|Vector|MakeVector (* _x (Variables|Default|GetColumn) 2.0) (* _y (Variables|Default|GetRow) 2.0) 0.0) :NewEnumerator1 (Math|Vector|MakeVector (Math|Float|SelectFloat _returnvalue_2 (+ _x _returnvalue_2) (== (Math|Integer|%(Integer) (Variables|Default|GetRow) 2) 0)) (* _y 2.0 (Variables|Default|GetRow) (/ 3.0 4.0)) 0.0) :NewEnumerator2 (Math|Vector|MakeVector (* _x 2.0 (Variables|Default|GetColumn) (/ 3.0 4.0)) (Math|Float|SelectFloat _returnvalue (+ _returnvalue _y) (== (Math|Integer|%(Integer) (Variables|Default|GetColumn) 2) 0)) 0.0))))

(fn CreateMID
  (bind _returnvalue (Rendering|Material|CreateDynamicMaterialInstance (Variables|Default|GetTile) 0 "/Game/Materials/Tiles/M_Tile.M_Tile" "None" :!class /Script/Engine.PrimitiveComponent))
  (bind _output_get (Variables|Internal│Material|SetMID _returnvalue))
  (Rendering|Material|SetVectorParameterValue _output_get "Color" (Variables|Default│Color|GetNormalColor) :!class /Script/Engine.MaterialInstanceDynamic))

(fn OnInteract
  (params (inSelect :type Boolean))
  (bind _mid (Variables|Internal│Material|GetMID)
    (:then
      (Rendering|Material|SetVectorParameterValue _mid "Color" (Math|Color|SelectColor (Variables|Default│Color|GetSelectedColor) (Variables|Default│Color|GetNormalColor) inSelect) :!class /Script/Engine.MaterialInstanceDynamic)
      (return true))
    (:else
      (return false))))