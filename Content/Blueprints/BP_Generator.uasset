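; BP_Generator is an actor that builds a grid of BP_TIle actors from its Rows and Columns settings.
; InitializeTiles first clears existing tiles, then spawns one tile per row and column at the generator's own transform, passing in the indices and calling each tile's Initialize.
; ClearTiles destroys every stored tile and empties the Tiles array.
; The event graph and construction script are empty, so nothing in this Blueprint calls InitializeTiles.
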(event EventBeginPlay)

(event Collision|EventActorBeginOverlap
  (params (OtherActor :type Actor%20Object%20Reference)))

(event EventTick
  (params (DeltaSeconds :type Float%20%28single-precision%29)))

(fn ConstructionScript)

(fn InitializeTiles
  (CallFunction|ClearTiles)
  (for _index (range 0 (- (Variables|Default|GetRows) 1))
    (for _index_2 (range 0 (- (Variables|Default|GetColumns) 1))
      (bind _returnvalue (Game|SpawnActorfromClass "/Game/Blueprints/BP_TIle.BP_TIle_C" (Math|Transform|MakeTransform (Transformation|GetActorLocation) (Transformation|GetActorRotation)) "AlwaysSpawn" "MultiplyWithRoot" self _index _index_2 0))
      (Default|Initialize _returnvalue)
      (Utilities|Array|Add (Variables|Default|GetTiles) _returnvalue))))

(fn ClearTiles
  (bind _tiles (Variables|Default|GetTiles))
  (if (> (Utilities|Array|Length (Variables|Default|GetTiles)) 0)
    (for _array_element _tiles
      (Actor|DestroyActor _array_element))
    (Utilities|Array|Clear _tiles)))